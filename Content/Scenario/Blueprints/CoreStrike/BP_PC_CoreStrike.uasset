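; Player controller for the CoreStrike scenario that requests player spawning and manages the end-of-game screen.
; On BeginPlay the local controller calls a server RPC, which asks BP_GM_CoreStrike to spawn its player.
; Opening the end screen removes any pause menu, shows UMG_GameEndMenu and switches to UI-only input with a visible, repositioned cursor.
; Closing it removes that menu and restores game-only input with the cursor hidden.
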(event Custom|RPC_Server_SpawnPlayer
  (bind _asbp_gm_core_strike (Utilities|Casting|CastToBP_GM_CoreStrike (Game|GetGameMode)))
  (Default|SpawnPlayer _asbp_gm_core_strike self))

(event Custom|Open%20End%20Screen
  (bind (_returnvalue _returnvalue2) (|GetWindowCenterPosition_2))
  ;[1 1 1] Remove Pause Screen, if open
  (bind _foundwidgets (Widget|GetAllWidgetsOfClass "/Game/Scenario/UI/UMG_PauseMenu.UMG_PauseMenu_C" true))
  (if (> (Utilities|Array|Length _foundwidgets) 0)
    (Widget|RemovefromParent (Utilities|Array|Get(acopy) _foundwidgets)))
  (bind _returnvalue_2 (UserInterface|CreateWidget "/Game/Scenario/UI/UMG_GameEndMenu.UMG_GameEndMenu_C"))
  (UserInterface|Viewport|AddtoViewport _returnvalue_2 2)
  (Class|PlayerController|SetMouseLocation _returnvalue _returnvalue2)
  (Input|SetInputModeUIOnly self _returnvalue_2 "DoNotLock")
  (Variables|Default|SetbShowMouseCursor true))

(event Custom|Close%20End%20Screen
  ;[1 1 1] Remove End Screen, if open
  (bind _foundwidgets (Widget|GetAllWidgetsOfClass "/Game/Scenario/UI/UMG_GameEndMenu.UMG_GameEndMenu_C" true))
  (if (> (Utilities|Array|Length _foundwidgets) 0)
    (Widget|RemovefromParent (Utilities|Array|Get(acopy) _foundwidgets)))
  (Input|SetInputModeGameOnly self)
  (Variables|Default|SetbShowMouseCursor false))

(event EventBeginPlay
  (if (Pawn|IsLocalController)
    (CallFunction|RPCServerSpawnPlayer)))

(fn ConstructionScript)