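; CoreStrike player state, judging by its name, that sets the player's username from saved player info.
; On BeginPlay it loads the save slot, caches it as a BP_Save_PlayerInfo, starts the username update and prints a debug message.
; The update chains an RPC-named event into a server-named one, which copies Username from its own cached save reference into PlayerUsername rather than receiving it as a parameter.
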(event Custom|RPC_UpdateUsername
  (CallFunction|RPCServerUpdateUsername))

(event Custom|RPC_Server_UpdateUsername
  (Variables|Default|SetPlayerUsername (Variables|/Game/Scenario/Blueprints/BP_Save_PlayerInfo.BP_Save_PlayerInfo_C|GetUsername (Variables|Default|GetSaveGame_Ref))))

(event EventBeginPlay
  (bind _returnvalue (SaveGame|LoadGamefromSlot (Variables|Default|GetSave%20Slot%20Name)))
  (bind _asbp_save_player_info (Utilities|Casting|CastToBP_Save_PlayerInfo _returnvalue))
  (Variables|Default|SetSaveGame_Ref _asbp_save_player_info)
  (CallFunction|RPCUpdateUsername)
  (Development|PrintString "Loaded Username" true true "(R=0.065688,G=1.000000,B=0.078990,A=1.000000)" 1e+01))

(fn ConstructionScript)