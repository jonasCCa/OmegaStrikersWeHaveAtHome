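; BP_SpeedOrb is a respawning pickup that grants a temporary speed upgrade to a FirstPersonCharacter that overlaps it.
; The server handles the overlap, skips characters already upgraded, calls SpeedUpgrade and despawns the orb.
; SetSpawned toggles sphere visibility and overlap events, and schedules the next spawn time on despawn.
; The orb starts despawned; Tick fills a progress-circle widget during the countdown and respawns it when time is up.
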(event OnComponentBeginOverlap(Sphere)
  (params (OverlappedComponent :type Primitive%20Component%20Object%20Reference) (OtherActor :type Actor%20Object%20Reference) (OtherComp :type Primitive%20Component%20Object%20Reference) (OtherBodyIndex :type Integer) (bFromSweep :type Boolean) (SweepResult :type Hit%20Result%20Structure%20%28by%20ref%29))
  (if (Variables|SpeedPickup|GetIsSpawned)
    (if (Networking|IsServer)
      (Development|PrintString "overlapping")
      (bind _asfirst_person_character (Utilities|Casting|CastToFirstPersonCharacter OtherActor))
      (if (not (Variables|/Game/FirstPersonBP/Blueprints/FirstPersonCharacter.FirstPersonCharacter_C|GetIsUpgraded _asfirst_person_character))
        (Default|SpeedUpgrade _asfirst_person_character (Variables|SpeedPickup|GetSpeed%20Multiplier) (Variables|SpeedPickup|GetMultiplier%20Duration))
        (CallFunction|SetSpawned false)))))

(event Custom|Set%20Spawned
  (params (New%20Value :type Boolean))
  (bind _sphere (Variables|Default|GetSphere))
  (Rendering|SetVisibility _sphere New%20Value true)
  (bind _output_get (Variables|/Script/Engine.PrimitiveComponent|SetbGenerateOverlapEvents _sphere New%20Value))
  (bind _output_get_2 (Variables|SpeedPickup|SetIsSpawned _output_get))
  (if _output_get_2
    (Default|SetPercentage (Variables|Default|GetProgress%20Circle) 1.0)
    (else
      (Variables|SpeedPickup|SetNext%20Spawn (+ (Math|DateTime|Now) (Math|Timespan|FromSeconds (Variables|SpeedPickup|GetSpawn%20Time)))))))

(event EventTick
  (params (DeltaSeconds :type Float%20%28single-precision%29))
  (if (not (Variables|SpeedPickup|GetIsSpawned))
    (if (>= (Math|DateTime|Now) (Variables|SpeedPickup|GetNext%20Spawn))
      (CallFunction|SetSpawned true)
      (else
        (Default|SetPercentage (Variables|Default|GetProgress%20Circle) (- 1.0 (/ (Math|Timespan|GetTotalSeconds (- (Variables|SpeedPickup|GetNext%20Spawn) (Math|DateTime|Now))) (Variables|SpeedPickup|GetSpawn%20Time))))))))

(event EventBeginPlay
  (bind _asumd_progress_circle (Utilities|Casting|CastToUMD_ProgressCircle (UserInterface|GetWidget (Variables|Default|GetProgress%20Bar))))
  (Variables|Default|SetProgress%20Circle _asumd_progress_circle)
  (CallFunction|SetSpawned false))

(fn ConstructionScript)