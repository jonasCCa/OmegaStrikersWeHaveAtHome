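; GoalHandler is a team goal that scores when an actor tagged Ball overlaps its box trigger.
; The overlap finds the MatchHandler through a class search and increases the score for the goal's TeamNumber.
; Barrier-break notifications recheck every goal barrier and open the goal door once all are broken.
; Resetting the goal restores each barrier and closes the door.
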(event OnComponentBeginOverlap(Box)
  (params (OverlappedComponent :type Primitive%20Component%20Object%20Reference) (OtherActor :type Actor%20Object%20Reference) (OtherComp :type Primitive%20Component%20Object%20Reference) (OtherBodyIndex :type Integer) (bFromSweep :type Boolean) (SweepResult :type Hit%20Result%20Structure%20%28by%20ref%29))
  (if (Actor|ActorHasTag OtherActor "Ball")
    (bind _outactors (Actor|GetAllActorsOfClass "/Game/Scenario/Blueprints/MatchHandler.MatchHandler_C"))
    (Default|IncreaseScore (Utilities|Array|Get(acopy) _outactors) (Variables|GoalHandler|GetTeam%20Number))))

(event Custom|Notify%20Broken%20Barrier
  (bind _array_element (Utilities|Array|ForEachLoopwithBreak (Variables|GoalHandler|GetGoalBarriers) :!label _label)
    (:LoopBody
      (if (Variables|/Game/Scenario/Blueprints/Barrier.Barrier_C|GetIsBroken _array_element)
        (Variables|GoalHandler|SetAllBarriersBroken true)
        (else
          (Variables|GoalHandler|SetAllBarriersBroken false)
          (goto _label Break))))
    (:Completed
      (if (Variables|GoalHandler|GetAllBarriersBroken)
        (Default|OpenDoor (Variables|GoalHandler|GetGoalDoor))))))

(event Custom|Reset%20Goal
  (for _array_element (Variables|GoalHandler|GetGoalBarriers)
    (Default|ResetBarrier _array_element)
    (Default|CloseDoor (Variables|GoalHandler|GetGoalDoor))))

(fn ConstructionScript)