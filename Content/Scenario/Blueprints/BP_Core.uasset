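; BP_Core is the physics-driven core that serves as the ball in a scoring game.
; ResetCore moves it back to the world X/Y origin at its current height and clears its linear velocity.
; SetInvisible and SetVisible toggle the mesh's visibility together with its overlap events.
; PlayScoreEffects spawns an electric destruction emitter at the core and plays the 2D goal sound.
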(event Custom|Play%20Score%20Effects
  (Effects|SpawnEmitteratLocation "/Game/Realistic_Starter_VFX_Pack_Vol2/Particles/Destruction/P_Destruction_Electric.P_Destruction_Electric" (Transformation|GetWorldLocation (Variables|Default|GetCore)) "0, 0, 0" "3.000000,3.000000,3.000000")
  (Audio|PlaySound2D "/Game/Scenario/SFX/Goal_SFX.Goal_SFX" 1.0 1.0 0.0 0 0))

(event Custom|Set%20Invisible
  (bind _core (Variables|Default|GetCore))
  (Rendering|SetVisibility _core false false)
  (Variables|/Script/Engine.PrimitiveComponent|SetbGenerateOverlapEvents _core false))

(event Custom|Set%20Visible
  (bind _core (Variables|Default|GetCore))
  (Rendering|SetVisibility _core true false)
  (Variables|/Script/Engine.PrimitiveComponent|SetbGenerateOverlapEvents _core true))

(event Custom|Reset%20Core
  (bind _core (Variables|Default|GetCore))
  (Transformation|SetWorldLocation _core (Math|Vector|MakeVector 0.0 0.0 (.z (Transformation|GetWorldLocation _core))) false false)
  (Physics|SetPhysicsLinearVelocity (Variables|Default|GetCore) "0, 0, 0" false "None") ; Reset Ball's Physics
)

(fn ConstructionScript)