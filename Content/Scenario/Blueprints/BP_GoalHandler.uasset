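; BP_GoalHandler manages one team's goal in Core Strike, handling scoring and the barriers that guard the goal door.
; When a BP_Core overlaps its box on the server, it tells the game mode to increase the opposing team's score.
; Broken-barrier notifications recheck all linked barriers and open the door once every one is broken.
; ResetGoal restores the barriers and closes the door.
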(event OnComponentBeginOverlap(Box)
  (params (OverlappedComponent :type Primitive%20Component%20Object%20Reference) (OtherActor :type Actor%20Object%20Reference) (OtherComp :type Primitive%20Component%20Object%20Reference) (OtherBodyIndex :type Integer) (bFromSweep :type Boolean) (SweepResult :type Hit%20Result%20Structure%20%28by%20ref%29))
  ;[1 1 1] Goal Scored
  (if (Networking|IsServer)
    (Utilities|Casting|CastToBP_Core OtherActor)
    (bind _asbp_gm_core_strike (Utilities|Casting|CastToBP_GM_CoreStrike (Game|GetGameMode)))
    (Default|IncreaseScore _asbp_gm_core_strike (Math|Integer|Absolute(Integer) (- (Variables|GoalHandler|GetTeam%20Number) 1)))))

(event Custom|Notify%20Broken%20Barrier
  (bind _array_element (Utilities|Array|ForEachLoopwithBreak (Variables|GoalHandler|GetGoalBarriers) :!label _label)
    (:LoopBody
      (if (Variables|/Game/Scenario/Blueprints/BP_GoalBarrier.BP_GoalBarrier_C|GetIsBroken _array_element)
        (Variables|GoalHandler|SetAllBarriersBroken true)
        (else
          (Variables|GoalHandler|SetAllBarriersBroken false)
          (goto _label Break))))
    (:Completed
      (if (Variables|GoalHandler|GetAllBarriersBroken)
        (Default|OpenDoor (Variables|GoalHandler|GetGoalDoor))))))

(event Custom|Reset%20Goal
  (for _array_element (Variables|GoalHandler|GetGoalBarriers)
    (Default|ResetBarrier _array_element)
    (Default|CloseDoor (Variables|GoalHandler|GetGoalDoor))))

(fn ConstructionScript)