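; BP_GoalBarrier is a breakable goal barrier that the ball, BP_Core, knocks out on contact.
; A server-only hit check on its Cube triggers HitByBall, which flags it broken, hides the actor, disables collision and notifies the GoalHandler.
; ResetBarrier clears the flag and restores visibility and collision, so the same actor is reused rather than destroyed.
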(event OnComponentHit(Cube)
  (params (HitComponent :type Primitive%20Component%20Object%20Reference) (OtherActor :type Actor%20Object%20Reference) (OtherComp :type Primitive%20Component%20Object%20Reference) (NormalImpulse :type Vector :default "0, 0, 0") (Hit :type Hit%20Result%20Structure%20%28by%20ref%29))
  ;[1 1 1] Hit By Ball
  (if (Networking|IsServer)
    (Utilities|Casting|CastToBP_Core OtherActor)
    (CallFunction|HitbyBall)))

(event Custom|Reset%20Barrier
  (Variables|Barrier|SetIsBroken false)
  (Rendering|SetActorHiddenInGame false)
  (Collision|SetCollisionEnabled (Variables|Default|GetCube) "QueryAndPhysics"))

(event Custom|HitByBall
  ;[1 1 1] Hit By Ball
  (Variables|Barrier|SetIsBroken true)
  (Rendering|SetActorHiddenInGame true)
  (Collision|SetCollisionEnabled (Variables|Default|GetCube) "NoCollision")
  (Default|NotifyBrokenBarrier (Variables|Default|GetGoalHandler)))

(event EventBeginPlay)

(fn ConstructionScript)