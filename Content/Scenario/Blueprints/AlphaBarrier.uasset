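; AlphaBarrier is a scenario trigger actor that toggles two team doors, Team1Door and Team2Door, together.
; Both hit and begin-overlap events on its Box component feed the same branch on an IsOpen flag, which opens or closes both doors and flips the flag.
; It does not filter which actor triggers it, so each hit or overlap toggles the doors again.
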(event OnComponentBeginOverlap(Box)
  (params (OverlappedComponent :type Primitive%20Component%20Object%20Reference) (OtherActor :type Actor%20Object%20Reference) (OtherComp :type Primitive%20Component%20Object%20Reference) (OtherBodyIndex :type Integer) (bFromSweep :type Boolean) (SweepResult :type Hit%20Result%20Structure%20%28by%20ref%29))
  (bind _team1_door (Variables|Default|GetTeam1_Door))
  (bind _team2_door (Variables|Default|GetTeam2_Door))
  (if (Variables|Default|GetIsOpen)
    (Default|CloseDoor _team1_door)
    (Default|CloseDoor _team2_door)
    (Variables|Default|SetIsOpen false)
    (else
      (Default|OpenDoor _team1_door)
      (Default|OpenDoor _team2_door)
      (Variables|Default|SetIsOpen true))))

(event OnComponentHit(Box)
  (params (HitComponent :type Primitive%20Component%20Object%20Reference) (OtherActor :type Actor%20Object%20Reference) (OtherComp :type Primitive%20Component%20Object%20Reference) (NormalImpulse :type Vector :default "0, 0, 0") (Hit :type Hit%20Result%20Structure%20%28by%20ref%29))
  (bind _team1_door (Variables|Default|GetTeam1_Door))
  (bind _team2_door (Variables|Default|GetTeam2_Door))
  (if (Variables|Default|GetIsOpen)
    (Default|CloseDoor _team1_door)
    (Default|CloseDoor _team2_door)
    (Variables|Default|SetIsOpen false)
    (else
      (Default|OpenDoor _team1_door)
      (Default|OpenDoor _team2_door)
      (Variables|Default|SetIsOpen true))))

(event EventBeginPlay)

(event Collision|EventActorBeginOverlap
  (params (OtherActor :type Actor%20Object%20Reference)))

(event EventTick
  (params (DeltaSeconds :type Float%20%28single-precision%29)))

(fn ConstructionScript)